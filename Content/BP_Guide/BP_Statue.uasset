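; BP_Statue is a collectible statue that jumps to random spots in the level until the player touches it.
; InitStatue teleports it within a fixed area at constant height, then re-arms a timer on itself with a delay that shrinks as the game mode's Level rises.
; On player overlap, unless the game is over, it reports to BP_Guide_GameMode, destroys itself and spawns a replacement, which relocates on BeginPlay.
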(event EventBeginPlay
  (bind _asbp_guide_game_mode (Utilities|Casting|CastToBP_Guide_GameMode (Game|GetGameMode)))
  (Variables|Default|SetMyGuideGameMode _asbp_guide_game_mode)
  (CallFunction|InitStatue))

(event Collision|EventActorBeginOverlap
  (params (OtherActor :type Actor%20Object%20Reference))
  (if (and (== (Game|GetPlayerCharacter 0) OtherActor) (not (Variables|/Game/BP_Guide/BP_Guide_GameMode.BP_Guide_GameMode_C|GetGameOver (Variables|Default|GetMyGuideGameMode))))
    (Default|StatueCollected (Variables|Default|GetMyGuideGameMode))
    (Actor|DestroyActor)
    (Game|SpawnActorfromClass "BP_Statue_C" (Transformation|GetActorTransform) "Undefined" 0 0)))

(event EventTick
  (params (DeltaSeconds :type Float%20%28single-precision%29)))

(fn ConstructionScript)

(fn InitStatue
  (Transformation|Teleport (Math|Vector|MakeVector (Math|Random|RandomFloatinRange -1.8e+03 1e+03) (Math|Random|RandomFloatinRange -1.8e+03 1e+03) 1.3e+02) "0, 0, 0")
  (Utilities|Time|SetTimerbyFunctionName 0 "InitStatue" (Math|Conversions|ToFloat(Integer) (- 6 (Variables|/Game/BP_Guide/BP_Guide_GameMode.BP_Guide_GameMode_C|GetLevel (Variables|Default|GetMyGuideGameMode))))))