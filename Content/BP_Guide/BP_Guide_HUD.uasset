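; BP_Guide_HUD is the guide game's HUD, showing score, time, player level and the game-over prompt.
; BeginPlay casts the game mode to BP_Guide_GameMode and caches it.
; DrawHUD draws the values read from that game mode as canvas text at fixed screen positions each frame.
; When the game mode's GameOver flag is set, it also draws "Game Over!" and "Press Enter".
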(event EventBeginPlay
  (bind _asbp_guide_game_mode (Utilities|Casting|CastToBP_Guide_GameMode (Game|GetGameMode)))
  (Variables|Default|SetMy_Guide_GameMode _asbp_guide_game_mode))

(event EventDrawHUD
  (params (SizeX :type Integer) (SizeY :type Integer))
  (bind _my_guide_gamemode (Variables|Default|GetMy_Guide_GameMode))
  (HUD|DrawText (Utilities|String|BuildString(Integer) "Score: " "" (Variables|/Game/BP_Guide/BP_Guide_GameMode.BP_Guide_GameMode_C|GetScore _my_guide_gamemode)) "(R=1.000000,G=0.846082,B=0.299910,A=1.000000)" 1e+01 1e+01 0 3.0 false)
  (HUD|DrawText (Utilities|String|BuildString(Integer) "Time: " "" (Variables|/Game/BP_Guide/BP_Guide_GameMode.BP_Guide_GameMode_C|GetTime _my_guide_gamemode)) "(R=1.000000,G=0.000000,B=0.075233,A=1.000000)" 3e+02 1e+01 0 3.0 false)
  (HUD|DrawText (Utilities|String|BuildString(Integer) "Player Level: " "" (Variables|/Game/BP_Guide/BP_Guide_GameMode.BP_Guide_GameMode_C|GetLevel _my_guide_gamemode)) "(R=1.000000,G=0.000000,B=0.075233,A=1.000000)" 5.5e+02 1e+01 0 3.0 false)
  (if (Variables|/Game/BP_Guide/BP_Guide_GameMode.BP_Guide_GameMode_C|GetGameOver (Variables|Default|GetMy_Guide_GameMode))
    (HUD|DrawText "Game Over!" "(R=1.000000,G=0.000000,B=0.075233,A=1.000000)" 4e+02 2e+02 0 3.0 false)
    (HUD|DrawText "Press Enter" "(R=1.000000,G=0.000000,B=0.075233,A=1.000000)" 4e+02 4e+02 0 3.0 false)))

(fn ConstructionScript)